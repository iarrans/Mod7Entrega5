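; NPC Blueprint that opens and closes dialogue as other actors enter and leave its trigger box.
; On begin overlap, an actor carrying a BP_DialogueComponent is passed to the NPC's dialogue component to begin dialogue, and GM_Gamemode's DialogueHUD is shown.
; End overlap ends dialogue and hides the HUD, but checks the NPC's own component rather than the departing actor's.
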(event OnComponentBeginOverlap(TriggerBox)
  (params (OverlappedComponent :type Primitive%20Component%20Object%20Reference) (OtherActor :type Actor%20Object%20Reference) (OtherComp :type Primitive%20Component%20Object%20Reference) (OtherBodyIndex :type Integer) (bFromSweep :type Boolean) (SweepResult :type Hit%20Result%20Structure%20%28by%20ref%29))
  (if (!= OtherActor self)
    (Utilities|IsValid (Actor|GetComponentbyClass OtherActor "/Game/Blueprints/Dialogue/BP_DialogueComponent.BP_DialogueComponent_C")
      (:Is%20Valid
        (Default|BeginDialogue (Variables|Default|GetBP_DialogueComponent) OtherActor)
        (bind _asgm_gamemode (Utilities|Casting|CastToGM_Gamemode (Game|GetGameMode)))
        (Widget|SetVisibility (Variables|/Game/Blueprints/GM_Gamemode.GM_Gamemode_C|GetDialogueHUD _asgm_gamemode) "Visible")))))

(event OnComponentEndOverlap(TriggerBox)
  (params (OverlappedComponent :type Primitive%20Component%20Object%20Reference) (OtherActor :type Actor%20Object%20Reference) (OtherComp :type Primitive%20Component%20Object%20Reference) (OtherBodyIndex :type Integer))
  (Utilities|IsValid (Actor|GetComponentbyClass "/Game/Blueprints/Dialogue/BP_DialogueComponent.BP_DialogueComponent_C")
    (:Is%20Valid
      (Default|EndDialogue (Variables|Default|GetBP_DialogueComponent) OtherActor)
      (bind _asgm_gamemode (Utilities|Casting|CastToGM_Gamemode (Game|GetGameMode)))
      (Widget|SetVisibility (Variables|/Game/Blueprints/GM_Gamemode.GM_Gamemode_C|GetDialogueHUD _asgm_gamemode) "Hidden"))))

(event EventBeginPlay)

(fn ConstructionScript)