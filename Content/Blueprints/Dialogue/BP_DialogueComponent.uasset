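; BP_DialogueComponent is a dialogue component for player and NPC actors that pairs two speakers and tracks their conversation state.
; BeginDialogue links both actors when started on the NPC, which runs its dialogue tree through AIC_NPCDialogue and notifies the partner.
; AdvanceDialogue forwards from player to NPC, whose controller advances the tree.
; EndDialogue accepts only the current partner, clears both sides and stops the NPC's brain logic.
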(event EventBeginPlay)

(event EventTick
  (params (DeltaSeconds :type Float%20%28single-precision%29)))

(fn BeginDialogue
  (params (ActorIn :type Actor%20Object%20Reference))
  (bind _returnvalue (Actor|GetComponentbyClass ActorIn "BP_DialogueComponent_C"))
  ;[1 1 1] Comprobamos que el otro actor tiene componente diálogo y que no hay conversación activa
  (Development|PrintText "Entra en Begin Dialogue")
  (if (and (Utilities|IsValid _returnvalue) (not (Variables|Default|GetTalking)))
    ;[1 1 1] Referencia  a actor conversación
    (Variables|Default|SetTalking true)
    (Variables|Default|SetOtherActor ActorIn)
    ;[1 1 1] soy npc?
    (if (not (Variables|Default|GetisPlayer))
      ;[1 1 1] si npc, behaviourtree
      (bind _asaic_npcdialogue (Utilities|Casting|CastToAIC_NPCDialogue (AI|GetAIController (Components|GetOwner))))
      (Default|BeginDialogueTree _asaic_npcdialogue)
      (CallFunction|BeginDialogue _returnvalue (Components|GetOwner)))))

(fn EndDialogue
  (params (ActorIn :type Actor%20Object%20Reference))
  ;[1 1 1] Para que no se creen referencias erróneas con un tercero
  (if (== ActorIn (Variables|Default|GetOtherActor))
    ;[1 1 1] Comprobamos que el otro actor tiene componente diálogo y estoy hablando
    (if (and (Utilities|IsValid (Actor|GetComponentbyClass ActorIn "BP_DialogueComponent_C")) (Variables|Default|GetTalking))
      ;[1 1 1] Limpiamos variables
      (Variables|Default|SetTalking false)
      (Variables|Default|SetOtherActor 0)
      (if (not (Variables|Default|GetisPlayer))
        (AI|Logic|StopLogic (Variables|/Script/AIModule.AIController|GetBrainComponent (AI|GetAIController (Components|GetOwner))) ""))
      ;[1 1 1] En ambos casos, paramos a nuestro interlocutor
      (CallFunction|EndDialogue (Actor|GetComponentbyClass ActorIn "BP_DialogueComponent_C") (Components|GetOwner)))))

(fn AdvanceDialogue
  (bind _otheractor (Variables|Default|GetOtherActor))
  (bind _returnvalue (Actor|GetComponentbyClass _otheractor "BP_DialogueComponent_C"))
  (Development|PrintString (Utilities|String|Append "isTalking" (Utilities|String|ToString(Boolean) (Variables|Default|GetTalking))) true true "(R=0.204041,G=0.000000,B=1.000000,A=1.000000)")
  ;[1 1 1] Si soy jugador y estoy hablando
  (if (Variables|Default|GetTalking)
    (if (Variables|Default|GetisPlayer)
      (Utilities|IsValid _otheractor ; Compruebo que tengo interlocutor
        (:Is%20Valid
          ;[1 1 1] Si interlocutor tiene componente diálogo, hago avanzar el diálogo del NPC
          (Utilities|IsValid _returnvalue
            (:Is%20Valid
              (CallFunction|AdvanceDialogue _returnvalue)
              (Development|PrintText "Advancing dialogue" true true "(R=1.000000,G=0.469855,B=0.000000,A=1.000000)")))))
      (else
        ;[1 1 1] Si es NPC, avanza en la conversación.
        (bind _asaic_npcdialogue (Utilities|Casting|CastToAIC_NPCDialogue (AI|GetAIController (Components|GetOwner))))
        (Default|AdvanceDialogueTree _asaic_npcdialogue)))))