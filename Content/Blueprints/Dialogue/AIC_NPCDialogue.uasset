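; AIC_NPCDialogue is an AI controller that drives NPC dialogue through a behavior tree.
; BeginDialogueTree runs the DialogueTree behavior tree.
; AdvanceDialogueTree sets the Interacted blackboard bool to true to signal the tree, with debug screen prints before and after the write.
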(event Custom|BeginDialogueTree
  (AI|RunBehaviorTree (Variables|Default|GetDialogueTree)))

(event Custom|AdvanceDialogueTree
  (bind _returnvalue (Utilities|Name|MakeLiteralName "Interacted"))
  (bind _blackboard (Variables|Default|GetBlackboard))
  (Development|PrintString "ENTERAAAA" true true "(R=1.000000,G=0.797618,B=0.000000,A=1.000000)")
  (AI|Components|Blackboard|SetValueasBool _blackboard _returnvalue true)
  (Development|PrintString (Utilities|String|Append "Interacted? " (Utilities|String|ToString(Boolean) (ScalableFloat|GetValueasBool _blackboard _returnvalue))) true true "(R=1.000000,G=0.000000,B=0.914603,A=1.000000)"))

(fn ConstructionScript)