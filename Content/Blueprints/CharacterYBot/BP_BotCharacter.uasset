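; BP_BotCharacter is the player character, handling camera-relative movement, sprint, crouch, jump, wall jumps, melee attack and dialogue advancing.
; Jumping while moving traces diagonally from the mesh for "Wall"-tagged actors, launching the character and setting side flags, once until landing.
; Left click plays a quick-attack montage with a one-second cooldown, and ToggleWeapon switches the child-actor weapon's collider.
; BeginPlay creates the HUD and links its health bar to the health component.
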(event EventBeginPlay
  ;[1 1 1] HUD
  (bind _returnvalue (UserInterface|CreateWidget "/Game/Blueprints/Combat/UMG_HUD.UMG_HUD_C"))
  (UserInterface|Viewport|AddtoViewport _returnvalue 0)
  (Variables|/Game/Blueprints/Combat/UMG_HealthBar.UMG_HealthBar_C|SetHealthComponent (Variables|/Game/Blueprints/Combat/UMG_HUD.UMG_HUD_C|GetUMG_HealthBar _returnvalue) (Variables|Default|GetBP_HealthComponent)))

(event EventOnLanded
  (params (Hit :type Hit%20Result%20Structure%20%28by%20ref%29))
  ;[1 1 1] Correr por la pared
  (Variables|Default|SetbLeftJump false)
  (Variables|Default|SetbRigthJump false)
  (Variables|Default|SetbCanWallJump true))

(event Input|ActionEvents|InputActionInteract
  (params (Key :type Key%20Structure :default "None"))
  ;[1 1 1] Avanzar diálogo
  (:Pressed
    (Development|PrintText "Llego a Interact")
    (Default|AdvanceDialogue (Variables|Default|GetBP_DialogueComponent))
    (Development|PrintString "Can Advance Dialogue")))

(event Input|ActionEvents|InputActionCrouch
  (params (Key :type Key%20Structure :default "None"))
  ;[1 1 1] agacharse
  (:Pressed
    (Character|Crouch))
  (:Released
    (Character|UnCrouch)))

(event Input|ActionEvents|InputActionCorrer
  (params (Key :type Key%20Structure :default "None"))
  ;[1 1 1] correr
  (:Pressed
    (Variables|/Script/Engine.CharacterMovementComponent|SetMaxWalkSpeed (Variables|Character|GetCharacterMovement) (Variables|Default|GetVelocidadCorrer)))
  (:Released
    (Variables|/Script/Engine.CharacterMovementComponent|SetMaxWalkSpeed (Variables|Character|GetCharacterMovement) 4e+02)))

(event Input|ActionEvents|InputActionJump
  (params (Key :type Key%20Structure :default "None"))
  (bind _mesh (Variables|Character|GetMesh))
  (bind _mesh_2 (Variables|Character|GetMesh))
  (bind _mesh_3 (Variables|Character|GetMesh))
  (bind _mesh_4 (Variables|Character|GetMesh))
  (bind _returnvalue (Transformation|GetWorldLocation _mesh_4))
  (bind _returnvalue_2 (Transformation|GetWorldLocation _mesh_2))
  ;[1 1 1] Correr por la pared
  (:Pressed
    (if (> (Math|Vector|VectorLength (Transformation|GetVelocity)) 0.0)
      (Utilities|FlowControl|Sequence
        (:then_0
          (bind (_outhit _returnvalue_3) (Collision|LineTraceByChannel _returnvalue_2 (+ _returnvalue_2 (* (+ (Math|Vector|GetForwardVector _mesh_2) (Math|Vector|GetRightVector _mesh_2)) 1e+02)) "TraceTypeQuery1" false 0 "ForOneFrame"))
          (if _returnvalue_3
            (if (Actor|ActorHasTag (.HitActor (Collision|BreakHitResult _outhit)) "Wall")
              (if (Variables|Default|GetbCanWallJump)
                (Variables|Default|SetbCanWallJump false)
                (Variables|Default|SetbLeftJump true)
                (Character|LaunchCharacter (Math|Vector|MakeVector 0.0 (.y (* (* (+ (Math|Vector|GetForwardVector _mesh_3) (Math|Vector|GetRightVector _mesh_3)) 8e+01) (.y (Transformation|GetActorScale3D (.HitActor (Collision|BreakHitResult _outhit)))))) 8e+02) false false)))))
        (:then_1
          (bind (_outhit_2 _returnvalue_4) (Collision|LineTraceByChannel _returnvalue (+ _returnvalue (* (+ (* (Math|Vector|GetForwardVector _mesh_4) -1.0) (Math|Vector|GetRightVector _mesh_4)) 1e+02)) "TraceTypeQuery1" false 0 "ForOneFrame" true "(R=0.980174,G=0.109634,B=1.000000,A=1.000000)"))
          (if _returnvalue_4
            (if (Actor|ActorHasTag (.HitActor (Collision|BreakHitResult _outhit_2)) "Wall")
              (if (Variables|Default|GetbCanWallJump)
                (Variables|Default|SetbCanWallJump false)
                (Variables|Default|SetbRigthJump true)
                (Character|LaunchCharacter (Math|Vector|MakeVector 0.0 (.y (* (* (+ (* (Math|Vector|GetForwardVector _mesh) -1.0) (Math|Vector|GetRightVector _mesh)) 8e+01) (.y (Transformation|GetActorScale3D)))) 8e+02) false false)))))))))

(event Input|ActionEvents|InputActionJump
  (params (Key :type Key%20Structure :default "None"))
  ;[1 1 1] saltar
  (:Pressed
    (Character|Jump)
    (Animation|StopAnimMontage "/Game/Blueprints/Combat/CombatAnims/QuickAttack_Montage.QuickAttack_Montage"))
  (:Released
    (Character|StopJumping)))

(event Input|AxisEvents|InputAxisTurnCamera
  (params (AxisValue :type Float%20%28single-precision%29))
  ;[1 1 1] movimiento
  (Pawn|Input|AddControllerYawInput AxisValue))

(event Input|AxisEvents|InputAxisCameraLookUp
  (params (AxisValue :type Float%20%28single-precision%29))
  ;[1 1 1] ROTACION CAMARA/PERSONAJE
  (Pawn|Input|AddControllerPitchInput AxisValue))

(event Input|AxisEvents|InputAxisForward
  (params (AxisValue :type Float%20%28single-precision%29))
  ;[1 1 1] movimiento
  (Pawn|Input|AddMovementInput (Math|Vector|GetForwardVector (Math|Rotator|MakeRotator 0.0 0.0 (.Yaw (Math|Rotator|BreakRotator (Pawn|GetControlRotation :!class /Script/Engine.Pawn))))) AxisValue false))

(event Input|AxisEvents|InputAxisHorizontal
  (params (AxisValue :type Float%20%28single-precision%29))
  ;[1 1 1] movimiento
  (Pawn|Input|AddMovementInput (Math|Vector|GetRightVector (Math|Rotator|MakeRotator 0.0 0.0 (.Yaw (Math|Rotator|BreakRotator (Pawn|GetControlRotation :!class /Script/Engine.Pawn))))) AxisValue false))

(event Input|MouseEvents|LeftMouseButton
  (params (Key :type Key%20Structure :default "None"))
  ;[1 1 1] ataque
  (:Pressed
    (Utilities|FlowControl|DoOnce false :!label _label
      (:Completed
        (Animation|PlayAnimMontage "/Game/Blueprints/Combat/CombatAnims/QuickAttack_Montage.QuickAttack_Montage" 1.0 "None")
        (Utilities|FlowControl|Delay 1.0)
        (goto _label Reset)))))

(fn ConstructionScript)

(fn ToggleWeapon
  (params (isHitting :type Boolean))
  (bind _asbp_weapon (Utilities|Casting|CastToBP_Weapon (Variables|/Script/Engine.ChildActorComponent|GetChildActor (Variables|Default|GetWeapon))))
  (Default|ToggleWeaponCollider _asbp_weapon isHitting))