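; Enemy actor with a health component and a health bar widget that appears only while a BP_BotCharacter is nearby.
; BeginPlay hides the widget and hands the health component to its UMG_HealthBar.
; SphereCollider overlap begin and end events show and hide the bar.
; Tick polls the component's IsDead flag, then turns on mesh physics and collision and destroys the actor after a short delay.
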(event OnComponentBeginOverlap(SphereCollider)
  (params (OverlappedComponent :type Primitive%20Component%20Object%20Reference) (OtherActor :type Actor%20Object%20Reference) (OtherComp :type Primitive%20Component%20Object%20Reference) (OtherBodyIndex :type Integer) (bFromSweep :type Boolean) (SweepResult :type Hit%20Result%20Structure%20%28by%20ref%29))
  (Utilities|Casting|CastToBP_BotCharacter OtherActor)
  (Rendering|SetVisibility (Variables|Default|GetWidget) true false))

(event OnComponentEndOverlap(SphereCollider)
  (params (OverlappedComponent :type Primitive%20Component%20Object%20Reference) (OtherActor :type Actor%20Object%20Reference) (OtherComp :type Primitive%20Component%20Object%20Reference) (OtherBodyIndex :type Integer))
  (Utilities|Casting|CastToBP_BotCharacter OtherActor)
  (Rendering|SetVisibility (Variables|Default|GetWidget) false false))

(event EventBeginPlay
  (bind _widget (Variables|Default|GetWidget))
  (Rendering|SetVisibility _widget false false)
  (bind _asumg_health_bar (Utilities|Casting|CastToUMG_HealthBar (UserInterface|GetWidget _widget)))
  (Variables|/Game/Blueprints/Combat/UMG_HealthBar.UMG_HealthBar_C|SetHealthComponent _asumg_health_bar (Variables|Default|GetBP_HealthComponent)))

(event EventTick
  (params (DeltaSeconds :type Float%20%28single-precision%29))
  (bind _mesh (Variables|Character|GetMesh))
  (if (Variables|/Game/Blueprints/Combat/BP_HealthComponent.BP_HealthComponent_C|GetisDead (Variables|Default|GetBP_HealthComponent))
    (Physics|SetSimulatePhysics _mesh true)
    (Collision|SetCollisionEnabled _mesh "QueryAndPhysics")
    (Utilities|FlowControl|Delay 1.2)
    (Actor|DestroyActor)))

(fn ConstructionScript)