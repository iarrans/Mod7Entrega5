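; BP_Weapon is a melee-style weapon actor that damages enemies its box collider overlaps.
; The collider starts disabled on BeginPlay and is switched on or off through ToggleWeaponCollider.
; On overlap, it casts the other actor to BP_Enemy and passes WeaponDamage to that enemy's health component.
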(event OnComponentBeginOverlap(BoxCollider)
  (params (OverlappedComponent :type Primitive%20Component%20Object%20Reference) (OtherActor :type Actor%20Object%20Reference) (OtherComp :type Primitive%20Component%20Object%20Reference) (OtherBodyIndex :type Integer) (bFromSweep :type Boolean) (SweepResult :type Hit%20Result%20Structure%20%28by%20ref%29))
  (bind _asbp_enemy (Utilities|Casting|CastToBP_Enemy OtherActor))
  (Default|ReceiveDamage (Variables|/Game/Blueprints/Combat/BP_Enemy.BP_Enemy_C|GetBP_HealthComponent _asbp_enemy) (Variables|Default|GetWeaponDamage)))

(event EventBeginPlay
  (CallFunction|ToggleWeaponCollider false))

(fn ConstructionScript)

(fn ToggleWeaponCollider
  (params (isActive :type Boolean))
  (bind _boxcollider (Variables|Default|GetBoxCollider))
  (if isActive
    (Collision|SetCollisionEnabled _boxcollider "QueryAndPhysics")
    (else
      (Collision|SetCollisionEnabled _boxcollider "NoCollision"))))