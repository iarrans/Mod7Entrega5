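; Actor health component that tracks current health and a dead state for combat.
; BeginPlay fills CurrentHealth from MaxHealth.
; ReceiveDamage subtracts damage while alive, clamps health at zero and sets IsDead on a lethal hit, ignoring later damage.
; It fires no death event or notification, and Tick is unused.
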(event EventBeginPlay
  (Variables|Default|SetCurrentHealth (Variables|Default|GetMaxHealth)))

(event EventTick
  (params (DeltaSeconds :type Float%20%28single-precision%29)))

(fn ReceiveDamage
  (params (dmg :type Float%20%28double-precision%29))
  (if (not (Variables|Default|GetisDead))
    (if (<= (- (Variables|Default|GetCurrentHealth) dmg) 0.0)
      (Variables|Default|SetCurrentHealth 0.0)
      (Variables|Default|SetisDead true)
      (else
        (Variables|Default|SetCurrentHealth (- (Variables|Default|GetCurrentHealth) dmg))))))